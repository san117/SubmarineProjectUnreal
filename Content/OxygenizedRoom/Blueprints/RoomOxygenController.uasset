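; RoomOxygenController is a manager that spreads oxygen between connected oxygenized rooms in the level.
; It gathers every room actor on BeginPlay, then on Tick, behind a frame-length Delay, loops through each room's connected-room set.
; Oxygen flows from any higher neighbour into the lower room at a transfer speed scaled by world delta time, with both levels clamped to a fixed range.
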(event `self.ReceiveBeginPlay`
  ;[1 1 1] Room Finder
  (bind _outactors (`GameplayStatics.GetAllActorsOfClass` "/Game/OxygenizedRoom/Blueprints/OxyneziedRoom.OxyneziedRoom_C"))
  (set `self.AllRooms` _outactors))

(event `self.ReceiveTick`
  (params (DeltaSeconds :type "Float (single-precision)"))
  (bind _returnvalue (* (`GameplayStatics.GetWorldDeltaSeconds`) (`self.OxygenTranferSpeed`)))
  ;[1 1 1] Oxygen comunication
  (`KismetSystemLibrary.Delay` DeltaSeconds)
  (for _array_element (`self.AllRooms`)
    (bind _result (`BlueprintSetLibrary.Set_ToArray` (`/Game/OxygenizedRoom/Blueprints/OxyneziedRoom.ConnectedRooms` _array_element)))
    (for _array_element_2 _result
      (if (> (`/Game/OxygenizedRoom/Blueprints/OxyneziedRoom.Oxygen` _array_element_2) (`/Game/OxygenizedRoom/Blueprints/OxyneziedRoom.Oxygen` _array_element))
        (set `/Game/OxygenizedRoom/Blueprints/OxyneziedRoom.Oxygen` (`KismetMathLibrary.FClamp` (- (`/Game/OxygenizedRoom/Blueprints/OxyneziedRoom.Oxygen` _array_element_2) _returnvalue) 0.0 100.0) _array_element_2)
        (set `/Game/OxygenizedRoom/Blueprints/OxyneziedRoom.Oxygen` (`KismetMathLibrary.FClamp` (+ (`/Game/OxygenizedRoom/Blueprints/OxyneziedRoom.Oxygen` _array_element) _returnvalue) 0.0 100.0) _array_element)))))

(fn `UserConstructionScript`)