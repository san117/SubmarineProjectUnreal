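; Oxygenated room actor that holds an oxygen supply, which drains while the first-person player is inside.
; Begin and end overlap events cast to FirstPersonCharacter and toggle an inside flag.
; While the flag is set, Tick subtracts delta time from the actor's own Oxygen value, clamped to a fixed range.
; The graph has no refill or depletion response.
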(event `self.ReceiveActorBeginOverlap`
  (params (OtherActor :type "Actor Object Reference"))
  (cast `/Game/FirstPersonBP/Blueprints/FirstPersonCharacter` OtherActor)
  (set `self.isPlayerInside` true))

(event `self.ReceiveActorEndOverlap`
  (params (OtherActor :type "Actor Object Reference"))
  (cast `/Game/FirstPersonBP/Blueprints/FirstPersonCharacter` OtherActor)
  (set `self.isPlayerInside` false))

(event `self.ReceiveTick`
  (params (DeltaSeconds :type "Float (single-precision)"))
  (if (`self.isPlayerInside`)
    (set `self.Oxygen` (`KismetMathLibrary.FClamp` (- (`self.Oxygen`) DeltaSeconds) 0.0 100.0))))

(fn `UserConstructionScript`)