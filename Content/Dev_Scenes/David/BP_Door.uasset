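; Door Blueprint that slides its small door mesh up and back down when DoorOC fires.
; Trigger overlap enables player 0's input on the actor, and end overlap disables it.
; DoorOC toggles DoorTF to play or reverse a timeline that lerps the mesh's relative location, using the actor's world location as the base.
; Rotation nodes and a second slide timeline from local zero are left unconnected.
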(event `self.ReceiveBeginPlay`
  ;[1 1 1] Root Door
)

(event `self.Trigger.OnComponentBeginOverlap`
  (params (OverlappedComponent :type "PrimitiveComponent Object Reference") (OtherActor :type "Actor Object Reference") (OtherComp :type "PrimitiveComponent Object Reference") (OtherBodyIndex :type Integer) (bFromSweep :type Boolean) (SweepResult :type "HitResult Structure (by ref)"))
  (`self.EnableInput` (`GameplayStatics.GetPlayerController` 0)))

(event `DoorOC`
  (bind _returnvalue (`self.K2_GetActorLocation`))
  (if (`self.Door TF`)
    (set `self.Door TF` false)
    ;[1 1 1] Slide Door
    (bind (_direction _newtrack_0) (`Timeline|Timeline_0` :!label _label)
      (:`Update`
        (`SceneComponent.K2_SetRelativeLocation` (`self.SM_Door_Small_A`) (`KismetMathLibrary.VLerp` _returnvalue (+ _returnvalue (0.0 0.0 280.0)) _newtrack_0) false false)))
    (else
      (set `self.Door TF` true)
      (goto _label :!via `Reverse`))))

(event `self.Trigger.OnComponentEndOverlap`
  (params (OverlappedComponent :type "PrimitiveComponent Object Reference") (OtherActor :type "Actor Object Reference") (OtherComp :type "PrimitiveComponent Object Reference") (OtherBodyIndex :type Integer))
  (`self.DisableInput` (`GameplayStatics.GetPlayerController` 0)))

(fn `UserConstructionScript`)